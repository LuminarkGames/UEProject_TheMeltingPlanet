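; Player character that casts terrain spells on a world of Hexa tiles.
; Destruct and Construct fire projectiles unless the cursor is over Water, then pulse CastSpell for the Anim BP and turn toward the cursor.
; Crush and Raise line-trace to the Hexa underfoot, lower or raise it, then update the camera.
; The controller's SkillManager supplies unlocks (Destruct needs none), level-indexed values and one shared cooldown per spell pair.
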(event EventBeginPlay
  ;[1 0.9804 0.498] My Game Mode
  (Variables|References|SetMyGameMode (.AsMy%20Game%20Mode (Utilities|Casting|CastToMyGameMode (Game|GetGameMode))))
  ;[1 0.9804 0.498] My Controller
  (Variables|References|SetMyController (.AsMy%20Controller (Utilities|Casting|CastToMyController (Game|GetPlayerController 0))))
  ;[1 0.9804 0.498] Camera
  (bind _outactors (Actor|GetAllActorsOfClass "/Game/Project/Blueprints/Camera/BP_Camera.BP_Camera_C"))
  (Variables|Default|SetCamera (Utilities|Array|Get(acopy) _outactors))
  ;[1 0.9804 0.498] Reference Manager
  (bind __referencer (Default|GetReferencer (Variables|References|GetMyController)))
  (Variables|References|SetReferencer __referencer))

(event Input|ActionEvents|InputActionSpell_Raise
  (params (Key :type Key%20Structure :default "None"))
  (bind _returnvalue (Transformation|GetActorLocation))
  (bind _returnvalue_2 (Game|GetPlayerController 0))
  (bind _mycontroller (Variables|References|GetMyController))
  (bind (_x _y) (Math|Vector|BreakVector _returnvalue))
  (bind _asmy_controller (Utilities|Casting|CastToMyController _returnvalue_2))
  (bind _skillmanager (Variables|/Game/Project/Blueprints/MyController.MyController_C|GetSkillManager _mycontroller))
  (bind _skillmanager_2 (Variables|/Game/Project/Blueprints/MyController.MyController_C|GetSkillManager _asmy_controller))
  (:Pressed
    ;[0.2314 0.6941 0.1882] Skill Value
    (if (Variables|/Game/Project/Blueprints/Manager/Skill/SkillManager.SkillManager_C|GetUnlock_CrushUp (Variables|/Game/Project/Blueprints/MyController.MyController_C|GetSkillManager (Variables|References|GetMyController)))
      ;[0.2314 0.6941 0.1882] Time Is Ready
      (if (<= (Variables|/Game/Project/Blueprints/Manager/Skill/SkillManager.SkillManager_C|GetTimeReady_Crush _skillmanager_2) (Utilities|Time|GetTimeSeconds))
        ;[0.3412 0.302 1] Skill Value
        (Variables|/Game/Project/Blueprints/Manager/Skill/SkillManager.SkillManager_C|SetTimeReady_Crush _skillmanager_2 (+ (Utilities|Array|Get(acopy) (Variables|/Game/Project/Blueprints/Manager/Skill/SkillManager.SkillManager_C|GetValue_Crush_Cooldown _skillmanager_2) (- (Variables|/Game/Project/Blueprints/Manager/Skill/SkillManager.SkillManager_C|GetLevel_Crush_Cooldown _skillmanager_2) 1)) (Utilities|Time|GetTimeSeconds)))
        ;[0.3412 0.302 1] Get the Hexa Below our Character
        (bind _outhit (Collision|LineTraceByChannel _returnvalue (Math|Vector|MakeVector _x _y 0.0) "TraceTypeQuery1" false 0 "None"))
        (if (== (Utilities|GetClass (.hitactor _outhit)) "/Game/Project/Blueprints/Manager/Hexa/Hexa.Hexa_C")
          ;[0.3412 0.302 1] Skill Value
          (Default|SpellConstruct (.AsHexa (Utilities|Casting|CastToHexa (.hitactor _outhit))) (Math|Float|Truncate (Utilities|Array|Get(acopy) (Variables|/Game/Project/Blueprints/Manager/Skill/SkillManager.SkillManager_C|GetValue_CrushUp_Damage _skillmanager) (- (Variables|/Game/Project/Blueprints/Manager/Skill/SkillManager.SkillManager_C|GetLevel_Crush_Cooldown _skillmanager) 1))) 0.0)
          ;[0.3882 0.8706 1] Move Camera
          (Default|KeysMoveFollowActor (Variables|Default|GetCamera)))))))

(event Input|ActionEvents|InputActionSpell_Crush
  (params (Key :type Key%20Structure :default "None"))
  (bind _returnvalue (Game|GetPlayerController 0))
  (bind _returnvalue_2 (Transformation|GetActorLocation))
  (bind _mycontroller (Variables|References|GetMyController))
  (bind (_x _y) (Math|Vector|BreakVector _returnvalue_2))
  (bind _asmy_controller (Utilities|Casting|CastToMyController _returnvalue))
  (bind _skillmanager (Variables|/Game/Project/Blueprints/MyController.MyController_C|GetSkillManager _mycontroller))
  (bind _skillmanager_2 (Variables|/Game/Project/Blueprints/MyController.MyController_C|GetSkillManager _asmy_controller))
  (:Pressed
    ;[0.2314 0.6941 0.1882] Skill Value
    (if (Variables|/Game/Project/Blueprints/Manager/Skill/SkillManager.SkillManager_C|GetUnlock_CrushDown (Variables|/Game/Project/Blueprints/MyController.MyController_C|GetSkillManager (Variables|References|GetMyController)))
      ;[0.2314 0.6941 0.1882] Time Is Ready
      (if (<= (Variables|/Game/Project/Blueprints/Manager/Skill/SkillManager.SkillManager_C|GetTimeReady_Crush _skillmanager_2) (Utilities|Time|GetTimeSeconds))
        ;[0.3412 0.302 1] Skill Value
        (Variables|/Game/Project/Blueprints/Manager/Skill/SkillManager.SkillManager_C|SetTimeReady_Crush _skillmanager_2 (+ (Utilities|Array|Get(acopy) (Variables|/Game/Project/Blueprints/Manager/Skill/SkillManager.SkillManager_C|GetValue_Crush_Cooldown _skillmanager_2) (- (Variables|/Game/Project/Blueprints/Manager/Skill/SkillManager.SkillManager_C|GetLevel_Crush_Cooldown _skillmanager_2) 1)) (Utilities|Time|GetTimeSeconds)))
        ;[0.3412 0.302 1] Get the Hexa Below our Character
        (bind _outhit (Collision|LineTraceByChannel _returnvalue_2 (Math|Vector|MakeVector _x _y 0.0) "TraceTypeQuery1" false 0 "None"))
        (if (== (Utilities|GetClass (.hitactor _outhit)) "/Game/Project/Blueprints/Manager/Hexa/Hexa.Hexa_C")
          ;[0.3412 0.302 1] Cast Spell on this Hexa
          (Default|SpellCrush (.AsHexa (Utilities|Casting|CastToHexa (.hitactor _outhit))) (Math|Float|Truncate (Utilities|Array|Get(acopy) (Variables|/Game/Project/Blueprints/Manager/Skill/SkillManager.SkillManager_C|GetValue_CrushDown_Damage _skillmanager) (- (Variables|/Game/Project/Blueprints/Manager/Skill/SkillManager.SkillManager_C|GetLevel_Crush_Cooldown _skillmanager) 1))))
          ;[0.3882 0.8706 1] Move Camera
          (Default|KeysMoveFollowActor (Variables|Default|GetCamera)))))))

(event Input|ActionEvents|InputActionSpell_Construct
  (params (Key :type Key%20Structure :default "None"))
  (bind _returnvalue (Game|GetPlayerController 0))
  (bind _returnvalue_2 (Game|GetPlayerCharacter 0))
  (bind _returnvalue_3 (Game|GetPlayerController 0))
  (bind _hitresult (Game|Player|GetHitResultUnderCursorbyChannel _returnvalue "TraceTypeQuery1" true))
  (bind _returnvalue_4 (Transformation|GetActorLocation _returnvalue_2))
  (bind _asmy_controller (Utilities|Casting|CastToMyController _returnvalue_3))
  (bind _location (Collision|BreakHitResult _hitresult))
  (bind _skillmanager (Variables|/Game/Project/Blueprints/MyController.MyController_C|GetSkillManager _asmy_controller))
  (bind (_x _y) (Math|Vector|BreakVector _location))
  (:Pressed
    ;[0.2314 0.6941 0.1882] Can't Cast on Water
    (if (!= (Utilities|GetClass (.HitActor (Collision|BreakHitResult (.HitResult (Game|Player|GetHitResultUnderCursorbyChannel (Game|GetPlayerController 0) "TraceTypeQuery1" true))))) "/Game/Project/Blueprints/Manager/Water/Water.Water_C")
      ;[0.2314 0.6941 0.1882] Ice Skill Unlocked
      (if (Variables|/Game/Project/Blueprints/Manager/Skill/SkillManager.SkillManager_C|GetUnlock_Ice (Variables|/Game/Project/Blueprints/MyController.MyController_C|GetSkillManager (Variables|References|GetMyController)))
        ;[0.2314 0.6941 0.1882] Time Is Ready
        (if (<= (Variables|/Game/Project/Blueprints/Manager/Skill/SkillManager.SkillManager_C|GetTimeReady_Spell _skillmanager) (Utilities|Time|GetTimeSeconds))
          ;[0.3412 0.302 1] Skill Value
          (Variables|/Game/Project/Blueprints/Manager/Skill/SkillManager.SkillManager_C|SetTimeReady_Spell _skillmanager (+ (Utilities|Array|Get(acopy) (Variables|/Game/Project/Blueprints/Manager/Skill/SkillManager.SkillManager_C|GetValue_Spell_Cooldown _skillmanager) (- (Variables|/Game/Project/Blueprints/Manager/Skill/SkillManager.SkillManager_C|GetLevel_Spell_Cooldown _skillmanager) 1)) (Utilities|Time|GetTimeSeconds)))
          ;[0.7216 0.1373 0.1294] Spawn Fire Spell
          (Game|SpawnActorfromClass "/Game/Project/Character/Spell/Bullet_Construct.Bullet_Construct_C" (Transformation|GetWorldTransform (Variables|Default|GetShoot)) "Undefined" 0 0)
          ;[0.3882 0.8706 1] Play Sound
          (Default|SoundPlay (.AsSound%20Manager (Utilities|Casting|CastToSoundManager (Variables|/Script/Engine.ChildActorComponent|GetChildActor (Variables|/Game/Project/Blueprints/MyController.MyController_C|GetSoundManager (.AsMy%20Controller (Utilities|Casting|CastToMyController (Game|GetPlayerController 0))))))) "NewEnumerator34" "0, 0, 0" true)
          ;[0.3412 0.302 1] Spell Animation (Animation BP)
          (Variables|Default|SetCastSpell true)
          (Utilities|FlowControl|Delay 0.1)
          (Variables|Default|SetCastSpell false)
          ;[0.3882 0.8706 1] Character Look the Spell Direction
          (Transformation|SetActorRotation _returnvalue_2 (Math|Rotator|FindLookatRotation _returnvalue_4 (Math|Vector|MakeVector _x _y (.Z (Math|Vector|BreakVector _returnvalue_4))))))))))

(event Input|ActionEvents|InputActionSpell_Destruct
  (params (Key :type Key%20Structure :default "None"))
  (bind _returnvalue (Game|GetPlayerController 0))
  (bind _returnvalue_2 (Game|GetPlayerCharacter 0))
  (bind _returnvalue_3 (Game|GetPlayerController 0))
  (bind _hitresult (Game|Player|GetHitResultUnderCursorbyChannel _returnvalue "TraceTypeQuery1" true))
  (bind _returnvalue_4 (Transformation|GetActorLocation _returnvalue_2))
  (bind _asmy_controller (Utilities|Casting|CastToMyController _returnvalue_3))
  (bind _location (Collision|BreakHitResult _hitresult))
  (bind _skillmanager (Variables|/Game/Project/Blueprints/MyController.MyController_C|GetSkillManager _asmy_controller))
  (bind (_x _y) (Math|Vector|BreakVector _location))
  (:Pressed
    ;[0.2314 0.6941 0.1882] Can't Cast on Water
    (if (!= (Utilities|GetClass (.HitActor (Collision|BreakHitResult (.HitResult (Game|Player|GetHitResultUnderCursorbyChannel (Game|GetPlayerController 0) "TraceTypeQuery1" true))))) "/Game/Project/Blueprints/Manager/Water/Water.Water_C")
      ;[0.2314 0.6941 0.1882] Time Is Ready
      (if (<= (Variables|/Game/Project/Blueprints/Manager/Skill/SkillManager.SkillManager_C|GetTimeReady_Spell _skillmanager) (Utilities|Time|GetTimeSeconds))
        ;[0.3412 0.302 1] Skill Value
        (Variables|/Game/Project/Blueprints/Manager/Skill/SkillManager.SkillManager_C|SetTimeReady_Spell _skillmanager (+ (Utilities|Array|Get(acopy) (Variables|/Game/Project/Blueprints/Manager/Skill/SkillManager.SkillManager_C|GetValue_Spell_Cooldown _skillmanager) (- (Variables|/Game/Project/Blueprints/Manager/Skill/SkillManager.SkillManager_C|GetLevel_Spell_Cooldown _skillmanager) 1)) (Utilities|Time|GetTimeSeconds)))
        ;[0.7216 0.1373 0.1294] Spawn Fire Spell
        (Game|SpawnActorfromClass "/Game/Project/Character/Spell/Bullet_Destruct.Bullet_Destruct_C" (Transformation|GetWorldTransform (Variables|Default|GetShoot)) "Undefined" 0 0)
        ;[0.3882 0.8706 1] Play Sound
        (Default|SoundPlay (.AsSound%20Manager (Utilities|Casting|CastToSoundManager (Variables|/Script/Engine.ChildActorComponent|GetChildActor (Variables|/Game/Project/Blueprints/MyController.MyController_C|GetSoundManager (.AsMy%20Controller (Utilities|Casting|CastToMyController (Game|GetPlayerController 0))))))) "NewEnumerator33" "0, 0, 0" true)
        ;[0.3412 0.302 1] Spell Animation (Animation BP)
        (Variables|Default|SetCastSpell true)
        (Utilities|FlowControl|Delay 0.1)
        (Variables|Default|SetCastSpell false)
        ;[0.3882 0.8706 1] Character Look the Spell Direction
        (Transformation|SetActorRotation _returnvalue_2 (Math|Rotator|FindLookatRotation _returnvalue_4 (Math|Vector|MakeVector _x _y (.Z (Math|Vector|BreakVector _returnvalue_4)))))))))

(fn ConstructionScript)