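; Game camera actor that follows the player character, another actor or a static mesh component, or moves to stored or given transforms.
; A mode-driven Tick eases toward the offset target or interpolates transforms over distance-based durations, with per-axis locks.
; Follow and move functions enable Tick on demand; key-follow mode ends once easing completes.
; It starts offset from the first PlayerStart and also supports direct, bounds-clamped key panning.
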(event Custom|Allow%20Camera%20Movement
  (params (_Delay :type Float%20%28single-precision%29)))

(event EventTick
  (params (DeltaSeconds :type Float%20%28single-precision%29))
  (bind _returnvalue (Transformation|GetActorLocation))
  (bind _returnvalue_2 (Transformation|GetActorLocation))
  ;[1 0 0.552] Tick Disabled at Start
  ; (Class Defaults Menu)
  (Variables|Default|SetDeltaSeconds DeltaSeconds)
  (switch Utilities|FlowControl|Switch|SwitchonE_CameraMode (Variables|Default|GetMode)
    (:NewEnumerator4
      ;[0.3412 0.302 1] Automatically Deactivate the Camera
      (Actor|Tick|SetActorTickEnabled false))
    (:NewEnumerator5
      ;[0.2314 0.6941 0.1882] We Focus a Component
      (if (Utilities|Enum|Equal(Enum) (Variables|Default|GetMode) "NewEnumerator6") :!label _label
        ;[0.3412 0.302 1] Update the Focus on the Character (or another object) to Manage the Inertia
        ; (The character will continue to walk after releasing the key, so we can't update the destination only when the key is pressed)
        (Variables|Default|SetLocation_Destination (+ (Transformation|GetWorldLocation (Variables|Default|GetFollow_StaticMeshComponent)) (Variables|Default|GetDistance_CameraActors)))
        (else
          (Variables|Default|SetLocation_Destination (+ (Transformation|GetActorLocation (Variables|Default|GetFollow_Actor)) (Variables|Default|GetDistance_CameraActors)))))
      ;[0.3412 0.302 1] Update Lerp Alpha Value
      (bind _output_get (Variables|Default|SetSmooth_LocationLerpAlpha (+ (Variables|Default|GetSmooth_LocationLerpAlpha) (Variables|Default|GetDeltaSeconds))))
      ;[0.3882 0.8706 1] Update Camera Location
      (Transformation|SetActorLocation self (Math|Vector|MakeVector (select (Variables|Default|GetVerrou_X) (.x _returnvalue_2) (.x (Math|Interpolation|Ease "EaseOut" (Math|Float|MapRangeUnclamped (Math|Float|Min(Float) _output_get (Variables|Default|GetParam_Move_Smooth_LocationDuration)) 0.0 (Variables|Default|GetParam_Move_Smooth_LocationDuration) 0.0 1.0) (Variables|Default|GetLocation_Start) (Variables|Default|GetLocation_Destination) 2.0))) (select (Variables|Default|GetVerrou_Y) (.y _returnvalue_2) (.y (Math|Interpolation|Ease "EaseOut" (Math|Float|MapRangeUnclamped (Math|Float|Min(Float) _output_get (Variables|Default|GetParam_Move_Smooth_LocationDuration)) 0.0 (Variables|Default|GetParam_Move_Smooth_LocationDuration) 0.0 1.0) (Variables|Default|GetLocation_Start) (Variables|Default|GetLocation_Destination) 2.0))) (select (Variables|Default|GetVerrou_Z) (.z _returnvalue_2) (.z (Math|Interpolation|Ease "EaseOut" (Math|Float|MapRangeUnclamped (Math|Float|Min(Float) _output_get (Variables|Default|GetParam_Move_Smooth_LocationDuration)) 0.0 (Variables|Default|GetParam_Move_Smooth_LocationDuration) 0.0 1.0) (Variables|Default|GetLocation_Start) (Variables|Default|GetLocation_Destination) 2.0)))) false false)
      ;[0.2314 0.6941 0.1882] Animation Finished
      (if (== (Math|Float|MapRangeUnclamped (Math|Float|Min(Float) _output_get (Variables|Default|GetParam_Move_Smooth_LocationDuration)) 0.0 (Variables|Default|GetParam_Move_Smooth_LocationDuration) 0.0 1.0) 1.0)
        ;[0.2314 0.6941 0.1882] We Can Deactivate the Camera If we use the Keys Because we will get Instructions When the Keys will again be Pressed
        (if (Utilities|Enum|Equal(Enum) (Variables|Default|GetMode) "NewEnumerator5")
          ;[0.3412 0.302 1] Stop the Animation
          (Variables|Default|SetMode "NewEnumerator4"))))
    (:NewEnumerator1
      (goto _label))
    (:NewEnumerator6
      (goto _label))
    (:NewEnumerator2
      ;[0.3412 0.302 1] Update Current Duration
      (bind _output_get_2 (Variables|Default|SetFollow_DurationCurrent (+ (Variables|Default|GetFollow_DurationCurrent) (Variables|Default|GetDeltaSeconds))))
      ;[0.3882 0.8706 1] Update Camera Location
      (Transformation|SetActorTransform (Math|Transform|MakeTransform (Math|Vector|MakeVector (select (Variables|Default|GetVerrou_X) (.x _returnvalue) (.x (.location (Math|Interpolation|Ease "EaseInOut" (Math|Float|Min(Float) (/ _output_get_2 (Variables|Default|GetFollow_DurationTotal)) 1.0) (Variables|Default|GetFollow_TransformStart) (Variables|Default|GetFollow_TransformDestination) 2.0)))) (select (Variables|Default|GetVerrou_Y) (.y _returnvalue) (.y (.location (Math|Interpolation|Ease "EaseInOut" (Math|Float|Min(Float) (/ _output_get_2 (Variables|Default|GetFollow_DurationTotal)) 1.0) (Variables|Default|GetFollow_TransformStart) (Variables|Default|GetFollow_TransformDestination) 2.0)))) (select (Variables|Default|GetVerrou_Z) (.z _returnvalue) (.z (.location (Math|Interpolation|Ease "EaseInOut" (Math|Float|Min(Float) (/ _output_get_2 (Variables|Default|GetFollow_DurationTotal)) 1.0) (Variables|Default|GetFollow_TransformStart) (Variables|Default|GetFollow_TransformDestination) 2.0))))) (.rotation (Math|Interpolation|Ease "EaseInOut" (Math|Float|Min(Float) (/ _output_get_2 (Variables|Default|GetFollow_DurationTotal)) 1.0) (Variables|Default|GetFollow_TransformStart) (Variables|Default|GetFollow_TransformDestination) 2.0)) (.scale (Math|Interpolation|Ease "EaseInOut" (Math|Float|Min(Float) (/ _output_get_2 (Variables|Default|GetFollow_DurationTotal)) 1.0) (Variables|Default|GetFollow_TransformStart) (Variables|Default|GetFollow_TransformDestination) 2.0))))
      ;[0.2314 0.6941 0.1882] Animation Finished
      (if (== (Math|Float|Min(Float) (/ _output_get_2 (Variables|Default|GetFollow_DurationTotal)) 1.0) 1.0)
        ;[0.3412 0.302 1] Stop the Animation
        (Variables|Default|SetMode "NewEnumerator4")))))

(event EventBeginPlay
  (Utilities|FlowControl|Sequence
    (:then_0
      ;[1 0.9804 0.498] My Character
      (Variables|References|SetMyCharacter (.AsMy%20Character (Utilities|Casting|CastToMyCharacter (Game|GetPlayerCharacter 0))))
      ;[1 0.9804 0.498] My Controller
      (Variables|References|SetMyController (.AsMy%20Controller (Utilities|Casting|CastToMyController (Game|GetPlayerController 0)))))
    (:then_1
      ;[0.3412 0.302 1] Init Actor to Follow
      (Variables|Default|SetFollow_Actor (Variables|References|GetMyCharacter))
      ;[0.3412 0.302 1] Init Initial Transform
      (Utilities|Map|Add (Variables|Default|GetDestination) "NewEnumerator9" (Transformation|GetActorTransform)))))

(fn ConstructionScript
  ;[0.3916 0.8714 1] Init Location
  (bind _outactors (Actor|GetAllActorsOfClass "/Script/Engine.PlayerStart"))
  (Transformation|SetActorLocation (+ (Transformation|GetActorLocation (Utilities|Array|Get(acopy) _outactors)) (Variables|Default|GetDistance_CameraActors)) false false)
  ;[0.3916 0.8714 1] Init Rotation
  (Transformation|SetActorRotation (Variables|Default|GetRotation_Origin)))

(fn KeysMoveFollowActor
  ;[1 0 0.552] The Main Difference with the KeysMove_OnlyCamera is that here we will Continue to Follow the Actor Even After Releasing the Keys, and Until the Actor Stop Moving
  ;[0.2314 0.6941 0.1882] Camera Not Free
  (if (not (Variables|Default|GetIsCameraFree))
    (Utilities|FlowControl|Sequence
      (:then_0
        (switch Utilities|FlowControl|Switch|SwitchonE_CameraMode (Variables|Default|GetMode)
          (:NewEnumerator4
            _)
          (:NewEnumerator5
            _))
        ;[0.3412 0.302 1] Next Location
        (Variables|Default|SetLocation_Destination (+ (Transformation|GetActorLocation (Variables|Default|GetFollow_Actor)) (Variables|Default|GetDistance_CameraActors)))
        ;[0.3412 0.302 1] Reset the Smoothness to Continue a little after Releasing the Moving Key
        (Variables|Default|SetLocation_Start (Transformation|GetActorLocation))
        (Variables|Default|SetSmooth_LocationLerpAlpha 0.0))
      (:then_1
        (switch Utilities|FlowControl|Switch|SwitchonE_CameraMode (Variables|Default|GetMode)
          (:NewEnumerator4
            ;[0.3412 0.302 1] Initialize
            (Variables|Default|SetMode "NewEnumerator5")
            (Actor|Tick|SetActorTickEnabled true)))))))

(fn KeysMoveDirectOnlyCamera
  (params (_SpeedForward :type Float%20%28single-precision%29) (_SpeedRight :type Float%20%28single-precision%29))
  (bind _returnvalue (Transformation|GetActorLocation))
  (bind _camerafree_limitmin (Variables|Default|GetCameraFree_LimitMin))
  (bind _camerafree_limitmax (Variables|Default|GetCameraFree_LimitMax))
  (if (and (or (!= _SpeedForward 0.0) (!= _SpeedRight 0.0)) (Variables|Default|GetAllowKeyMove))
    ;[0.3882 0.8706 1] Camera Location
    (Transformation|SetActorLocation (Math|Vector|MakeVector (Math|Float|Clamp(Float) (+ (.x _returnvalue) (* _SpeedRight (Variables|Default|GetSpeed))) (.x _camerafree_limitmin) (.x _camerafree_limitmax)) (Math|Float|Clamp(Float) (+ (.y _returnvalue) (* _SpeedForward (Variables|Default|GetSpeed))) (.y _camerafree_limitmin) (.y _camerafree_limitmax)) (.z _returnvalue)) false false)
    (Variables|Default|SetMode "NewEnumerator1")))

(fn MovetoDestination
  (params (_Destination :type E_CameraDestination%20Enum :default "NewEnumerator8") (_IgnoreRotation :type Boolean) (_MoveDirect :type Boolean))
  (bind _destination (Variables|Default|GetDestination))
  (bind _value (Utilities|Map|Find _destination _Destination))
  ;[0.3412 0.302 1] Move to the Destination
  ; We May Ignore the Rotation in Parameter to Keep the Camera One
  (bind __delay (MoveTo|MovetoTransform (Math|Transform|MakeTransform (.location _value) (select _IgnoreRotation (Transformation|GetActorRotation) (.rotation _value)) "1,1,1") _MoveDirect))
  (return __delay))

(fn MovetoLocation
  (params (_Location :type Vector) (_MoveDirect :type Boolean))
  (bind __delay (MoveTo|MovetoTransform (Math|Transform|MakeTransform _Location (Transformation|GetActorRotation) "1,1,1") _MoveDirect))
  (return __delay))

(fn MovetoTransform
  (params (_Destination :type Transform) (_MoveDirect :type Boolean))
  (bind _returnvalue (Transformation|GetActorLocation))
  (Development|PrintString "-- Move to Transform")
  (Development|PrintString (Utilities|String|ToString(Vector) (.location _Destination)))
  (Development|PrintString (Utilities|String|ToString(Vector) _returnvalue))
  ;[0.2314 0.6941 0.1882] Not to the Same Place
  (if (Math|Vector|NotEqual(Vector) (.location _Destination) _returnvalue 0.0001)
    ;[0.2314 0.6941 0.1882] Move Direct Without Smooth Animation
    (if _MoveDirect
      ;[0.3916 0.8714 1] Teleport Direct the Camera
      (Transformation|SetActorTransform _Destination false true)
      (else
        ;[0.3412 0.302 1] Transform
        (bind _output_get (Variables|Default|SetFollow_TransformDestination _Destination))
        (Development|PrintString (Utilities|String|ToString(Transform) _output_get))
        (bind _output_get_2 (Variables|Default|SetFollow_TransformStart (Transformation|GetActorTransform)))
        (Development|PrintString (Utilities|String|ToString(Transform) _output_get_2))
        (Variables|Default|SetMode "NewEnumerator2")
        (Variables|Default|SetFollow_DurationCurrent 0.0)
        ;[0.3412 0.302 1] Duration
        (bind _output_get_3 (Variables|Default|SetFollow_DurationTotal (/ (Math|Vector|VectorLength (- (.location (Variables|Default|GetFollow_TransformDestination)) (.location (Variables|Default|GetFollow_TransformStart)))) (/ (Variables|Default|GetSpeed_Auto) 2.0))))
        (Development|PrintString (Utilities|String|ToString(Float) _output_get_3))
        (Actor|Tick|SetActorTickEnabled true)
        (return _output_get_3)))))

(fn ResetLocation
  (params (_ForceToFollowCharacter :type Boolean))
  ;[0.3916 0.8714 1] Init Location
  (Transformation|SetActorLocation (+ (Transformation|GetActorLocation (Variables|Default|GetFollow_Actor)) (Variables|Default|GetDistance_CameraActors)) false false)
  ;[0.3916 0.8714 1] Init Rotation
  (Transformation|SetActorRotation (Variables|Default|GetRotation_Origin)))

(fn FollowFollowActor
  (params (_Actor :type Actor%20Object%20Reference))
  (Variables|Default|SetFollow_Actor (select (Utilities|IsValid _Actor) _Actor (Game|GetPlayerCharacter 0)))
  (Variables|Default|SetMode "NewEnumerator1")
  (Variables|Default|SetLocation_Start (Transformation|GetActorLocation))
  (Variables|Default|SetSmooth_LocationLerpAlpha 0.0)
  (Variables|Default|SetFollow_DurationCurrent 0.0)
  ;[0.3412 0.302 1] Duration
  (Variables|Default|SetFollow_DurationTotal (/ (Math|Vector|VectorLength (- (Transformation|GetActorLocation (Variables|Default|GetFollow_Actor)) (Transformation|GetActorLocation))) (/ (Variables|Default|GetSpeed) 2.0)))
  (Actor|Tick|SetActorTickEnabled true))

(fn FollowFollowStaticMeshComponent
  (params (_StaticMeshComponent :type Static%20Mesh%20Component%20Object%20Reference))
  (Variables|Default|SetFollow_StaticMeshComponent _StaticMeshComponent)
  (Variables|Default|SetMode "NewEnumerator6")
  (Variables|Default|SetLocation_Start (Transformation|GetActorLocation))
  (Variables|Default|SetSmooth_LocationLerpAlpha 0.0)
  (Variables|Default|SetFollow_DurationCurrent 0.0)
  ;[0.3412 0.302 1] Duration
  (Variables|Default|SetFollow_DurationTotal (/ (Math|Vector|VectorLength (- (Transformation|GetWorldLocation (Variables|Default|GetFollow_StaticMeshComponent)) (Transformation|GetActorLocation))) (/ (Variables|Default|GetSpeed) 2.0)))
  (Actor|Tick|SetActorTickEnabled true))

(fn FollowStopFollow
  (Variables|Default|SetMode "NewEnumerator4"))