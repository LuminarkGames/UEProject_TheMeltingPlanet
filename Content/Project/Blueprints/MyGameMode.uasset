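; MyGameMode is a game mode Blueprint that runs the startup sequence on BeginPlay.
; It polls with short delays until the player controller is valid, then caches the BP_Camera actor, MyController and its WidgetManager.
; It then polls the controller's SaveMenuManager until initialization finishes, before toggling the main interface through WidgetManager and calling the SaveManager's Manager function.
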(event EventBeginPlay
  (Utilities|FlowControl|Delay 0.01)
  ;[0.3412 0.302 1] Wait the Controller Loading
  (Utilities|IsValid (Game|GetPlayerController 0) :!label _label
    (:Is%20Valid
      (Utilities|FlowControl|Sequence
        (:then_0
          ;[1 0.9804 0.498] Camera
          (bind _outactors (Actor|GetAllActorsOfClass "/Game/Project/Blueprints/Camera/BP_Camera.BP_Camera_C"))
          (Variables|References|SetCamera (Utilities|Array|Get(acopy) _outactors))
          ;[1 0.9804 0.498] MyController
          (Variables|References|SetMyController (.AsMy%20Controller (Utilities|Casting|CastToMyController (Game|GetPlayerController 0))))
          ;[1 0.9804 0.498] Widget Manager
          (Variables|References|SetWidgetManager (Variables|/Game/Project/Blueprints/MyController.MyController_C|GetWidgetManager (Variables|References|GetMyController))))
        (:then_1
          ;[0.3412 0.302 1] Wait the Controller Loading
          (if (not (Variables|/Game/Project/Blueprints/Manager/Save/SaveMenuManager.SaveMenuManager_C|GetInitDone (Variables|/Game/Project/Blueprints/MyController.MyController_C|GetSaveMenuManager (Variables|References|GetMyController)))) :!label _label_2
            (Utilities|FlowControl|Delay 0.01)
            (goto _label_2)
            (else
              ;[0.3882 0.8706 1] Display Main Interface
              (Default|ToggleWidget (Variables|/Game/Project/Blueprints/MyController.MyController_C|GetWidgetManager (Variables|References|GetMyController)) "NewEnumerator0" "NewEnumerator0")
              (Default|Manager (Variables|/Game/Project/Blueprints/MyController.MyController_C|GetSaveManager (Variables|References|GetMyController))))))))
    (:Is%20Not%20Valid
      (Utilities|FlowControl|Delay 0.01)
      (goto _label))))

(fn ConstructionScript)